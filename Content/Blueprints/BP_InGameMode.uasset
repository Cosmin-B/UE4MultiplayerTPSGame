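; In-game game mode that spawns enemy bots and awards score when a player is killed.
; SpawnNewBot runs an EQS query for spawn locations, then spawns a randomly chosen BP_AdvancedAI or BP_TrackerBot at each returned point, at roughly even odds.
; An actor-killed delegate, bound on BeginPlay, adds score to the killer's CSPlayerState when the victim is player-controlled and the killer still has a valid pawn.
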(event `self.ReceiveBeginPlay`
  (add `self.OnActorKilled` (delegate `OnActorKilled_Event_0`)))

(event `self.SpawnNewBot`
  (bind _returnvalue (`EnvQueryManager.RunEQSQuery` "/Game/Blueprints/AI/EQS/EQS_FindSpawnLocation.EQS_FindSpawnLocation" self "RandomBest25Pct"))
  (add `EnvQueryInstanceBlueprintWrapper.OnQueryFinishedEvent` _returnvalue (delegate `OnQueryFinishedEvent_Event_0`)))

(event `OnActorKilled_Event_0` :!signature `self.OnActorKilled`
  (params (Victim :type "Actor Object Reference") (Killer :type "Actor Object Reference") (KillerController :type "Controller Object Reference"))
  (bind _returnvalue (`Controller.K2_GetPawn` KillerController))
  (bind _aspawn (cast `Pawn` Victim))
  (if (`Pawn.IsPlayerControlled` _aspawn)
    (`/Engine/EditorBlueprintResources/StandardMacros.IsValid` _returnvalue
      (:`Is Valid`
        (bind _ascsplayer_state (cast `CSPlayerState` (`Pawn.PlayerState` _returnvalue)))
        (`CSPlayerState.AddScore` _ascsplayer_state 20.0)))))

(event `OnQueryFinishedEvent_Event_0`
  (params (QueryInstance :type "EnvQueryInstanceBlueprintWrapper Object Reference") (QueryStatus :type "EEnvQueryStatus Enum" :default "Processing"))
  (switch `EEnvQueryStatus` QueryStatus
    (:`Success`
      (bind _resultlocations (`EnvQueryInstanceBlueprintWrapper.GetQueryResultsAsLocations` QueryInstance))
      (for _array_element _resultlocations
        (`|SpawnActorFromClass` (select `bool` (<= (`KismetMathLibrary.RandomFloatInRange` 0.0 100.0) 50.0) :`false` "/Game/Blueprints/AI/BP_TrackerBot.BP_TrackerBot_C" :`true` "/Game/Blueprints/AI/BP_AdvancedAI.BP_AdvancedAI_C" :!type "Actor Class Reference") (`KismetMathLibrary.MakeTransform` _array_element) "AdjustIfPossibleButDontSpawnIfColliding" "OverrideRootScale" null null)))))

(fn `UserConstructionScript`)