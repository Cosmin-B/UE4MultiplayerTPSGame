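; Blueprint function library of shared helpers for a co-op game, giving typed access to core classes and control of the mouse cursor.
; Two getters cast the game instance and a supplied player controller to BP_GameInstance and BP_PlayerController.
; ToggleCursor uses the controller getter to show a grab-hand cursor with mouse lock, or hide and unlock it, setting Game and UI input mode in both cases.
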(fn `GetCoopPlayerController`
  (params (InPlayerController :type "PlayerController Object Reference"))
  (returns (CoopPlayerController :type "/Game/Blueprints/Player/BP_PlayerController Object Reference"))
  (bind _asbp_player_controller (cast `/Game/Blueprints/Player/BP_PlayerController` InPlayerController))
  (return _asbp_player_controller))

(fn `GetGameInstanceBP`
  (returns (MyGameInstance :type "/Game/Blueprints/BP_GameInstance Object Reference"))
  (return (cast `/Game/Blueprints/BP_GameInstance` (`GameplayStatics.GetGameInstance` null) :!pure true)))

(fn `ToggleCursor`
  (params (bLock :type Boolean) (InPlayerController :type "PlayerController Object Reference"))
  (bind _coopplayercontroller (`self.GetCoopPlayerController` InPlayerController InPlayerController))
  (`PlayerController.SetMouseCursorWidget` _coopplayercontroller (select `bool` bLock :`true` "GrabHand" :!type "EMouseCursor Enum") null)
  (set `PlayerController.bShowMouseCursor` bLock _coopplayercontroller)
  (`WidgetBlueprintLibrary.SetInputMode_GameAndUIEx` _coopplayercontroller null (select `bool` bLock :`false` "DoNotLock" :`true` "LockAlways" :!type "EMouseLockMode Enum")))