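; Player HUD that shows the in-game widget and swaps in a statistics screen after each round.
; On BeginPlay it creates WBP_InGame and binds to CSGameState match-state changes.
; Each state change removes any existing statistics widget, and the Post Round state creates and shows a new WBP_Statistics.
; Tick polls the in-game widget's weapon info to update the ammo display every frame.
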(event `self.ReceiveBeginPlay`
  (bind _returnvalue (`|CreateWidget` "/Game/Blueprints/HUD/WBP/WBP_InGame.WBP_InGame_C" (`self.GetOwningPlayerController`)))
  (bind _output_get (set `self.InGameWidget` _returnvalue))
  (`UserWidget.AddToViewport` _output_get 0)
  (bind _ascsgame_state (cast `CSGameState` (`GameplayStatics.GetGameState`)))
  (add `CSGameState.OnMatchStateChanged` _ascsgame_state (delegate `OnMatchStateChanged_Event_0`)))

(event `OnMatchStateChanged_Event_0`
  (params (PreviousMatchState :type Name) (NewMatchState :type Name))
  (`|ExecutionSequence`
    (:`then_0`
      (`/Engine/EditorBlueprintResources/StandardMacros.IsValid` (`self.StatisticsWidget`)
        (:`Is Valid`
          (`Widget.RemoveFromParent` (`self.StatisticsWidget`)))))
    (:`then_1`
      (switch `name` NewMatchState
        (:`PostRound`
          (bind _returnvalue (`|CreateWidget` "/Game/Blueprints/HUD/WBP/WBP_Statistics.WBP_Statistics_C" (`self.GetOwningPlayerController`)))
          (bind _output_get (set `self.StatisticsWidget` _returnvalue))
          (`UserWidget.AddToViewport` _output_get 0))))))

(event `self.ReceiveTick`
  (params (DeltaSeconds :type "Float (single-precision)"))
  (bind _ingamewidget (`self.InGameWidget`))
  (`/Engine/EditorBlueprintResources/StandardMacros.IsValid` _ingamewidget
    (:`Is Valid`
      (`/Game/Blueprints/HUD/WBP/WBP_WeaponInfo.UpdateWeaponAmmo` (`/Game/Blueprints/HUD/WBP/WBP_InGame.WBP_WeaponInfo` _ingamewidget)))))

(fn `UserConstructionScript`)